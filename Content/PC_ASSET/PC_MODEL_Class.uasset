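; PC_MODEL_Class is an actor that displays a spinning Cube component with a detail widget that reacts to overlaps.
; Tick adds a small fixed local yaw rotation to the cube each frame, independent of delta time.
; Beginning and ending an overlap both toggle the Widget component's visibility, with no filter on the overlapping actor.
; On begin overlap it also casts the widget to detail_UI and copies MessageMain into its Messagepc.
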(event `self.ReceiveTick`
  (params (DeltaSeconds :type "Float (single-precision)"))
  (`SceneComponent.K2_AddLocalRotation` (`self.Cube`) (struct :`Yaw` 0.5) false false))

(event `self.ReceiveActorBeginOverlap`
  (params (OtherActor :type "Actor Object Reference"))
  (`SceneComponent.ToggleVisibility` (`self.Widget`) false)
  (bind _asdetail_ui (cast `/Game/PC_ASSET/detail_UI` (`WidgetComponent.GetWidget` (`self.Widget`))))
  (set `/Game/PC_ASSET/detail_UI.Messagepc` (`self.message_main`) _asdetail_ui))

(event `self.ReceiveBeginPlay`)

(event `self.ReceiveActorEndOverlap`
  (params (OtherActor :type "Actor Object Reference"))
  (`SceneComponent.ToggleVisibility` (`self.Widget`) false))

(fn `UserConstructionScript`)